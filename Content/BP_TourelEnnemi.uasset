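; Enemy turret that aims and fires at the player while the player is inside its Zone trigger.
; Tick yaws the Capsule and pitches the Canon toward the player via look-at rotations, with a Delay in Tick pacing BP_BulletEnnemi spawns at the Arrow.
; Damage lowers Health, destroying the turret at exactly zero, otherwise briefly swapping Canon and Base materials to blue before setting them red.
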(event OnComponentBeginOverlap(Zone)
  (params (OverlappedComponent :type Primitive%20Component%20Object%20Reference) (OtherActor :type Actor%20Object%20Reference) (OtherComp :type Primitive%20Component%20Object%20Reference) (OtherBodyIndex :type Integer) (bFromSweep :type Boolean) (SweepResult :type Hit%20Result%20Structure%20%28by%20ref%29))
  ;[1 1 1] Player in zone
  (if (== OtherActor (Game|Player|GetPlayerPawn 0))
    (Variables|Default|SetIsInTriggerZone true)))

(event OnComponentEndOverlap(Zone)
  (params (OverlappedComponent :type Primitive%20Component%20Object%20Reference) (OtherActor :type Actor%20Object%20Reference) (OtherComp :type Primitive%20Component%20Object%20Reference) (OtherBodyIndex :type Integer))
  ;[1 1 1] Player exit zone
  (if (== OtherActor (Game|Player|GetPlayerPawn 0))
    (Variables|Default|SetIsInTriggerZone false)))

(event EventBeginPlay)

(event Collision|EventActorBeginOverlap
  (params (OtherActor :type Actor%20Object%20Reference)))

(event EventTick
  (params (DeltaSeconds :type Float%20%28single-precision%29))
  (bind _arrow (Variables|Default|GetArrow))
  ;[1 1 1] Movement Turret
  (if (Variables|Default|GetIsInTriggerZone)
    (Transformation|SetWorldRotation (Variables|Default|GetCapsule) (CallFunction|RotationTurret DeltaSeconds) false false)
    (Transformation|SetWorldRotation (Variables|Default|Getcanon) (CallFunction|RotationCanon DeltaSeconds) false false)
    (Utilities|FlowControl|Delay 2.0)
    (Game|SpawnActorfromClass "/Game/Blueprints/Projectile/BP_BulletEnnemi.BP_BulletEnnemi_C" (Math|Transform|MakeTransform (Transformation|GetWorldLocation _arrow) (Transformation|GetWorldRotation _arrow) "1,1,1") "Undefined" 0 0)))

(event Game|Damage|EventAnyDamage
  (params (Damage :type Float%20%28single-precision%29) (DamageType :type Damage%20Type%20Object%20Reference) (InstigatedBy :type Controller%20Object%20Reference) (DamageCauser :type Actor%20Object%20Reference))
  ;[1 1 1] Get Damage
  (bind _output_get (Variables|Default|SetHealth (- (Variables|Default|GetHealth) (Math|Float|Truncate Damage))))
  (if (== _output_get 0)
    (Actor|DestroyActor)
    (else
      (Rendering|Material|SetMaterial (Variables|Default|Getcanon) 1 "/Game/Materials/ColorMaterialsInstances/MI_ColorBlu.MI_ColorBlu")
      (Utilities|FlowControl|Delay 0.5)
      (Rendering|Material|SetMaterial (Variables|Default|Getcanon) 1 "/Game/Materials/ColorMaterialsInstances/MI_ColorRed.MI_ColorRed"))))

(fn ConstructionScript)

(fn RotationTurret
  (params (DeltaTime :type Float%20%28single-precision%29))
  (bind _base (Variables|Default|Getbase))
  (bind _returnvalue (Transformation|GetWorldRotation _base))
  (bind (_roll _pitch) (Math|Rotator|BreakRotator _returnvalue))
  (return (Math|Interpolation|RInterpTo (Transformation|GetWorldRotation (Variables|Default|GetCapsule)) (Math|Rotator|MakeRotator _roll _pitch (.Yaw (Math|Rotator|BreakRotator (Math|Rotator|FindLookatRotation (Transformation|GetWorldLocation (Variables|Default|Getbase)) (Transformation|GetActorLocation (Game|Player|GetPlayerPawn 0)))))) DeltaTime 0.0)))

(fn RotationCanon
  (params (DeltaTime :type Float%20%28single-precision%29))
  (bind _capsule (Variables|Default|GetCapsule))
  (bind _returnvalue (Transformation|GetWorldRotation _capsule))
  (bind (_roll _pitch _yaw) (Math|Rotator|BreakRotator _returnvalue))
  (return (Math|Interpolation|RInterpTo (Transformation|GetWorldRotation (Variables|Default|Getcanon)) (Math|Rotator|MakeRotator _roll (.Pitch (Math|Rotator|BreakRotator (Math|Rotator|FindLookatRotation (Transformation|GetWorldLocation (Variables|Default|Getcanon)) (Transformation|GetActorLocation (Game|Player|GetPlayerPawn 0))))) _yaw) DeltaTime 0.0)))