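; Hover turret enemy that is visible and active only during its assigned game phase, and is destroyed once the phase passes.
; An optional timeline slides it to a destination, while Tick turns support and canon toward the player with RInterpTo and fires bullets, throttled by a Delay.
; Damage flashes its material blue; at zero or less health it simulates physics, awarding GameInstance score only on exactly zero.
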(event EventBeginPlay
  ;[1 1 1] Set movement ennemis
  (bind _asgame_instance_player (Utilities|Casting|CastToGameInstance_Player (Game|GetGameInstance)))
  (Variables|Default|SetAs%20Game%20Instance%20Player _asgame_instance_player)
  (if (Variables|Default|Getmovable)
    (Variables|Default|SetInitLocation (Transformation|GetWorldLocation (Variables|Default|GetStatic_HoverChassis)))
    (bind _moving (Timeline|movement Play)
      (:Update
        (Transformation|SetWorldLocation (Variables|Default|GetStatic_HoverChassis) (Math|Vector|Lerp(Vector) (Variables|Default|GetInitLocation) (Variables|Default|GetDestination) _moving) false false)))))

(event EventTick
  (params (DeltaSeconds :type Float%20%28single-precision%29))
  (bind _arrow (Variables|Default|GetArrow))
  (bind _static_hoverchassis (Variables|Default|GetStatic_HoverChassis))
  ;[1 1 1] Ennemis movement
  (if (CallFunction|CheckPhase)
    (Rendering|SetVisibility _static_hoverchassis true true)
    (if (Variables|Default|GetIsDead)
      ;[1 1 1] Set movement ennemis
      (bind _moving (Timeline|movement Stop)
        (:Update
          (Transformation|SetWorldLocation (Variables|Default|GetStatic_HoverChassis) (Math|Vector|Lerp(Vector) (Variables|Default|GetInitLocation) (Variables|Default|GetDestination) _moving) false false)))
      (else
        (Transformation|SetWorldRotation (Variables|Default|Getsupport) (CallFunction|SetRotationTurret DeltaSeconds) false false)
        (Transformation|SetWorldRotation (Variables|Default|Getcanon) (CallFunction|SetRotationCanon DeltaSeconds) false false)
        (Utilities|FlowControl|Delay 2.0)
        (if (not (Variables|Default|GetIsDead))
          (Game|SpawnActorfromClass "/Game/Blueprints/Projectile/BP_BulletEnnemi.BP_BulletEnnemi_C" (Math|Transform|MakeTransform (Transformation|GetWorldLocation _arrow) (Transformation|GetWorldRotation _arrow) "1,1,1") "Undefined" 0 0))))
    (else
      (Rendering|SetVisibility _static_hoverchassis false true)
      (if (> (Variables|/Game/Blueprints/Gameinstance/GameInstance_Player.GameInstance_Player_C|GetPhase (Variables|Default|GetAs%20Game%20Instance%20Player)) (Variables|Default|GetwhichPhase))
        (Actor|DestroyActor)))))

(event Game|Damage|EventAnyDamage
  (params (Damage :type Float%20%28single-precision%29) (DamageType :type Damage%20Type%20Object%20Reference) (InstigatedBy :type Controller%20Object%20Reference) (DamageCauser :type Actor%20Object%20Reference))
  ;[1 1 1] Ennemis Hit
  (bind _output_get (Variables|Default|SetHealth (- (Variables|Default|GetHealth) (Math|Float|Truncate Damage))))
  (if (<= _output_get 0)
    (Variables|Default|SetIsDead true)
    (Physics|SetSimulatePhysics (Variables|Default|GetStatic_HoverChassis) true)
    (Rendering|Material|SetMaterial (Variables|Default|Getcanon) 1 0)
    (if (== (Variables|Default|GetHealth) 0)
      (bind _asgame_instance_player (Utilities|Casting|CastToGameInstance_Player (Game|GetGameInstance)))
      (Variables|/Game/Blueprints/Gameinstance/GameInstance_Player.GameInstance_Player_C|SetScore _asgame_instance_player (+ (Variables|/Game/Blueprints/Gameinstance/GameInstance_Player.GameInstance_Player_C|GetScore _asgame_instance_player) 2e+02)))
    (else
      (Rendering|Material|SetMaterial (Variables|Default|Getcanon) 1 "/Game/Materials/ColorMaterialsInstances/MI_ColorBlu.MI_ColorBlu")
      (Utilities|FlowControl|Delay 0.2)
      (Rendering|Material|SetMaterial (Variables|Default|Getcanon) 1 "/Game/Materials/ColorMaterialsInstances/MI_ColorRed.MI_ColorRed"))))

(fn ConstructionScript)

(fn SetRotationTurret
  (params (DeltaTime :type Float%20%28single-precision%29))
  (bind _support (Variables|Default|Getsupport))
  (bind _returnvalue (Transformation|GetWorldRotation _support))
  (bind (_roll _pitch) (Math|Rotator|BreakRotator _returnvalue))
  (return (Math|Interpolation|RInterpTo (Transformation|GetWorldRotation (Variables|Default|Getbody)) (Math|Rotator|MakeRotator _roll _pitch (.Yaw (Math|Rotator|BreakRotator (Math|Rotator|FindLookatRotation (Transformation|GetWorldLocation (Variables|Default|Getsupport)) (Transformation|GetActorLocation (Game|Player|GetPlayerPawn 0)))))) DeltaTime 0.0)))

(fn SetRotationCanon
  (params (DeltaTime :type Float%20%28single-precision%29))
  (bind _support (Variables|Default|Getsupport))
  (bind _returnvalue (Transformation|GetWorldRotation _support))
  (bind (_roll _pitch _yaw) (Math|Rotator|BreakRotator _returnvalue))
  (return (Math|Interpolation|RInterpTo (Transformation|GetWorldRotation (Variables|Default|Getcanon)) (Math|Rotator|MakeRotator _roll (.Pitch (Math|Rotator|BreakRotator (Math|Rotator|FindLookatRotation (Transformation|GetWorldLocation (Variables|Default|Getcanon)) (Transformation|GetActorLocation (Game|Player|GetPlayerPawn 0))))) _yaw) DeltaTime 0.0)))

(fn CheckPhase
  (return (== (Variables|/Game/Blueprints/Gameinstance/GameInstance_Player.GameInstance_Player_C|GetPhase (Variables|Default|GetAs%20Game%20Instance%20Player)) (Variables|Default|GetwhichPhase))))