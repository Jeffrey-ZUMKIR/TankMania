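; BP_Collectable is a rotating pickup that awards score when it takes damage.
; On BeginPlay, a Turn timeline drives a rotator lerp that spins the Cube component through a full turn.
; Any damage adds a fixed amount to Score on GameInstance_Player and destroys the actor; overlap plays no part in collection.
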(event EventBeginPlay
  (bind _turn (Timeline|turn Play)
    (:Update
      (Transformation|SetRelativeLocationAndRotation (Variables|Default|GetCube) "0, 0, 0" (Math|Rotator|Lerp(Rotator) "0, 0, 0" "0,360.000000, 0" _turn) false false))))

(event Collision|EventActorBeginOverlap
  (params (OtherActor :type Actor%20Object%20Reference)))

(event EventTick
  (params (DeltaSeconds :type Float%20%28single-precision%29)))

(event Game|Damage|EventAnyDamage
  (params (Damage :type Float%20%28single-precision%29) (DamageType :type Damage%20Type%20Object%20Reference) (InstigatedBy :type Controller%20Object%20Reference) (DamageCauser :type Actor%20Object%20Reference))
  (bind _asgame_instance_player (Utilities|Casting|CastToGameInstance_Player (Game|GetGameInstance)))
  (Variables|/Game/Blueprints/Gameinstance/GameInstance_Player.GameInstance_Player_C|SetScore _asgame_instance_player (+ (Variables|/Game/Blueprints/Gameinstance/GameInstance_Player.GameInstance_Player_C|GetScore _asgame_instance_player) 30))
  (Actor|DestroyActor))

(fn ConstructionScript)