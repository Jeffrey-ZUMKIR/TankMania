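; BP_BulletPlayer is a player bullet that destroys itself three seconds after it spawns.
; On a blocking sphere hit it applies damage to the other actor and destroys itself.
; When the hit actor is a BP_BulletEnnemi, it instead turns on bouncing in its projectile movement, so it does no damage and survives.
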(event OnComponentHit(Sphere1)
  (params (HitComponent :type Primitive%20Component%20Object%20Reference) (OtherActor :type Actor%20Object%20Reference) (OtherComp :type Primitive%20Component%20Object%20Reference) (NormalImpulse :type Vector :default "0, 0, 0") (Hit :type Hit%20Result%20Structure%20%28by%20ref%29))
  (bind (_bblockinghit _binitialoverlap _time _distance _location _impactpoint _normal _impactnormal _physmat _hitactor) (Collision|BreakHitResult Hit))
  (if _bblockinghit
    (if (== (Utilities|GetClass _hitactor) "/Game/Blueprints/Projectile/BP_BulletEnnemi.BP_BulletEnnemi_C")
      (Variables|/Script/Engine.ProjectileMovementComponent|SetbShouldBounce (Variables|Default|GetProjectileMovement) true)
      (else
        (Game|Damage|ApplyDamage OtherActor 1.0 0 0)
        (Actor|DestroyActor)))))

(event EventBeginPlay
  (Utilities|FlowControl|Delay 3.0)
  (Actor|DestroyActor))

(event Collision|EventActorBeginOverlap
  (params (OtherActor :type Actor%20Object%20Reference)))

(event EventTick
  (params (DeltaSeconds :type Float%20%28single-precision%29)))

(fn ConstructionScript)